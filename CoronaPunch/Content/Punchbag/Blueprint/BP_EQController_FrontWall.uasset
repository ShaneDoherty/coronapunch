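; Audio visualizer controller that builds a front wall of cubes which pulse with the frequency spectrum of a track.
; On BeginPlay it spawns BP_Cube actors in a square grid on the XZ plane, then shuffles the array to scatter the bands.
; Each Tick samples the Track's spectrum at game time, one band per cube, and scales each cube's Y by its magnitude.
; Its Audio Play call is unconnected, so it starts no playback.
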(event EventBeginPlay
  (CallFunction|SpawnGrid)
  (Utilities|Array|Shuffle (Variables|Default|GetBP_CubeArray)))

(event Collision|EventActorBeginOverlap
  (params (OtherActor :type Actor%20Object%20Reference)))

(event EventTick
  (params (DeltaSeconds :type Float%20%28single-precision%29))
  (bind _outspectrum (Class|SoundVisualizationStatics|CalculateFrequencySpectrum (Variables|Default|GetTrack) 0 (Utilities|Time|GetGameTimeinSeconds) 0.1 (Utilities|Array|Length (Variables|Default|GetBP_CubeArray))))
  (Variables|Default|SetSpectrum _outspectrum)
  (for (_array_element _array_index) (Variables|Default|GetBP_CubeArray)
    (Transformation|SetActorScale3D _array_element (Math|Vector|MakeVector 1.0 (* (Math|Float|Absolute(Float) (Utilities|Array|Get(acopy) (Variables|Default|GetSpectrum) _array_index)) 0.02) 1.0))))

(fn ConstructionScript)

(fn SpawnGrid
  (params (NewParam :type Transform))
  (bind _distance (Variables|Default|GetDistance))
  (for _index (range 0 (- (Variables|Default|GetNumberOfCubes) 1))
    (bind _returnvalue (Game|SpawnActorfromClass "/Game/Punchbag/Blueprint/BP_Cube.BP_Cube_C" (Math|Transform|MakeTransform (Math|Vector|MakeVector (+ (* (Variables|Default|GetRow) _distance) (Variables|Default|GetF_X_Location)) (Variables|Default|GetF_Y_Location) (+ (* (Variables|Default|GetCol) _distance) (Variables|Default|GetF_Z_Location))) "0, 0, 0" "1,1,1") "AlwaysSpawn" 0 0))
    (Utilities|Array|Add (Variables|Default|GetBP_CubeArray) _returnvalue)
    (Math|Integer|IncrementInt (Variables|Default|GetRow)
      (:%20%20
        (if (== (Variables|Default|GetRow) (Math|Float|Truncate (Math|Float|Sqrt (Math|Conversions|ToFloat(Integer) (Variables|Default|GetNumberOfCubes)))))
          (Math|Integer|IncrementInt (Variables|Default|GetCol)
            (:%20%20
              (Variables|Default|SetRow 0))))))))